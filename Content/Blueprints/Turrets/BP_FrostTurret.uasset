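; Frost turret that slows and periodically damages BP_MoveChar characters within its detection sphere.
; Entering adds a character to the target array, halves its walk speed and sets a looping one-second Shoot timer that damages all targets.
; DoOnce stores the timer handle and deals an immediate hit on first entry only.
; Leaving removes the target and doubles its speed, but clears the timer when targets remain, not when empty.
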(event `self.ReceiveBeginPlay`
  (`KismetArrayLibrary.Array_Clear` (`self.TargetsArray`)))

(event `self.DetectionSphere.OnComponentBeginOverlap`
  (params (OverlappedComponent :type "PrimitiveComponent Object Reference") (OtherActor :type "Actor Object Reference") (OtherComp :type "PrimitiveComponent Object Reference") (OtherBodyIndex :type Integer) (bFromSweep :type Boolean) (SweepResult :type "HitResult Structure (by ref)"))
  (bind _asbp_move_char (cast `/Game/Blueprints/BP_MoveChar` OtherActor))
  (`KismetArrayLibrary.Array_Add` (`self.TargetsArray`) _asbp_move_char)
  (bind _charactermovement (`Character.CharacterMovement` _asbp_move_char))
  (set `CharacterMovementComponent.MaxWalkSpeed` (/ (`MovementComponent.GetMaxSpeed` _charactermovement) 2.0) _charactermovement)
  (bind _returnvalue (`KismetSystemLibrary.K2_SetTimerDelegate` (delegate `Shoot`) 1.0 true))
  (`/Engine/EditorBlueprintResources/StandardMacros.DoOnce` false
    (:`Completed`
      (set `self.TimerShoot` _returnvalue)
      (for _array_element (`self.TargetsArray`) :!label _label
        (`self.UpdateHealth` _array_element (`self.Damage`))))))

(event `Shoot`
  (goto _label))

(event `self.DetectionSphere.OnComponentEndOverlap`
  (params (OverlappedComponent :type "PrimitiveComponent Object Reference") (OtherActor :type "Actor Object Reference") (OtherComp :type "PrimitiveComponent Object Reference") (OtherBodyIndex :type Integer))
  (bind _asbp_move_char (cast `/Game/Blueprints/BP_MoveChar` OtherActor))
  (`KismetArrayLibrary.Array_RemoveItem` (`self.TargetsArray`) _asbp_move_char)
  (bind _charactermovement (`Character.CharacterMovement` _asbp_move_char))
  (set `CharacterMovementComponent.MaxWalkSpeed` (* (`MovementComponent.GetMaxSpeed` _charactermovement) 2.0) _charactermovement)
  (if (`KismetArrayLibrary.Array_IsNotEmpty` (`self.TargetsArray`))
    (`KismetSystemLibrary.K2_ClearAndInvalidateTimerHandle` (`self.TimerShoot`))))

(fn `UserConstructionScript`
  (`SphereComponent.SetSphereRadius` (`self.DetectionSphere`) (`self.RadiusDetection_0`) true))