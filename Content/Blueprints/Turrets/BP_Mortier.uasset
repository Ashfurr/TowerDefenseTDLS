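; Mortar turret that automatically fires on BP_MoveChar characters entering its detection sphere, whose radius is set in the construction script.
; Overlaps maintain a target array, and DetectAndShoot picks the closest entry when acquiring a target.
; A looping fire-rate timer line-traces toward the target, then spawns a following mortar projectile.
; Projectile and immediate damage go to the array entry at CurrentIndex, which this graph never updates.
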(event `self.ReceiveBeginPlay`
  (`KismetArrayLibrary.Array_Clear` (`self.TargetsArray`)))

(event `Shoot`
  (bind _output (`|GetArrayItem` (`self.TargetsArray`) (`self.CurrentIndex`)))
  (if (not (`KismetSystemLibrary.K2_IsTimerActiveHandle` (`self.TimerShoot`)))
    (bind _returnvalue (`KismetSystemLibrary.K2_SetTimerDelegate` (delegate `Projectil`) (`self.FireRate_0`) true))
    (`/Engine/EditorBlueprintResources/StandardMacros.DoOnce` false
      (:`Completed`
        (set `self.TimerShoot` _returnvalue)
        (if (`self.HasTarget`) :!label _label
          (bind _outhit (`KismetSystemLibrary.LineTraceSingle` :`Start` (`SceneComponent.K2_GetComponentLocation` (`self.Spawn`)) :`End` (`self.K2_GetActorLocation` (`self.Target`)) :`TraceChannel` "TraceTypeQuery1" :`DrawDebugType` "ForDuration"))
          (cast `/Game/Blueprints/BP_MoveChar` (`.HitActor` (`GameplayStatics.BreakHitResult` _outhit)))
          (bind _returnvalue_2 (`|SpawnActorFromClass` "/Game/Blueprints/Turrets/Projectiles/Bp_MortarProjectil.Bp_MortarProjectil_C" (`SceneComponent.K2_GetComponentToWorld` (`self.Spawn`)) "AdjustIfPossibleButAlwaysSpawn" "OverrideRootScale" null null))
          (`/Game/Blueprints/Turrets/Projectiles/Bp_MortarProjectil.Follow` _returnvalue_2 _output)
          (`/Game/Blueprints/IaGestion.UpdateHealth` _output (`self.Damage`)))))))

(event `Projectil`
  (goto _label))

(event `self.DetectionSphere.OnComponentBeginOverlap`
  (params (OverlappedComponent :type "PrimitiveComponent Object Reference") (OtherActor :type "Actor Object Reference") (OtherComp :type "PrimitiveComponent Object Reference") (OtherBodyIndex :type Integer) (bFromSweep :type Boolean) (SweepResult :type "HitResult Structure (by ref)"))
  (bind _targetsarray (`self.TargetsArray`))
  (bind _asbp_move_char (cast `/Game/Blueprints/BP_MoveChar` OtherActor))
  (bind _returnvalue (`KismetArrayLibrary.Array_Add` _targetsarray _asbp_move_char))
  (message `/Game/Blueprints/IaGestion.SetID` (`|GetArrayItem` _targetsarray _returnvalue) _returnvalue)
  (if (not (`self.HasTarget`))
    (`self.DetectAndShoot`)))

(event `self.DetectionSphere.OnComponentEndOverlap`
  (params (OverlappedComponent :type "PrimitiveComponent Object Reference") (OtherActor :type "Actor Object Reference") (OtherComp :type "PrimitiveComponent Object Reference") (OtherBodyIndex :type Integer))
  (bind _asbp_move_char (cast `/Game/Blueprints/BP_MoveChar` OtherActor))
  (if (== (`/Game/Blueprints/BP_MoveChar.Index` (`self.Target`)) (`/Game/Blueprints/BP_MoveChar.Index` _asbp_move_char))
    (`KismetArrayLibrary.Array_Remove` (`self.TargetsArray`))
    (if (`KismetArrayLibrary.Array_IsNotEmpty` (`self.TargetsArray`))
      (`self.DetectAndShoot`)
      (else
        (set `self.HasTarget` false)))
    (else
      (`KismetArrayLibrary.Array_RemoveItem` (`self.TargetsArray`) _asbp_move_char))))

(fn `DetectAndShoot`
  (bind _closeactor (`self.DetectCloser`))
  (set `self.Target` _closeactor)
  (`self.Shoot`)
  (set `self.HasTarget` true))

(fn `DetectCloser`
  (returns (CloseActor :type "/Game/Blueprints/BP_MoveChar Object Reference"))
  (locals (TempDist :type "Float (double-precision)" :default 9999999.0) (ReturnIndex :type Integer))
  (bind _targetsarray (`self.TargetsArray`))
  (set `local.TempDist` 99999.0)
  (if (> (`KismetArrayLibrary.Array_Length` _targetsarray) 1)
    (for (_array_element _array_index) _targetsarray
      (bind _returnvalue (`self.GetDistanceTo` _array_element self))
      (if (< _returnvalue (`local.TempDist`))
        (set `local.TempDist` _returnvalue)
        (set `local.ReturnIndex` _array_index)))
    (return (`|GetArrayItem` (`self.TargetsArray`) (`local.ReturnIndex`)))
    (else
      (return (`|GetArrayItem` (`self.TargetsArray`))))))

(fn `UserConstructionScript`
  (`SphereComponent.SetSphereRadius` (`self.DetectionSphere`) (`self.RadiusDetection_0`) true))