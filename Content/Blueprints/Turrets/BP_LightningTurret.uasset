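; Lightning turret that attacks several BP_MoveChar targets at once within a detection sphere sized at construction.
; Overlap events maintain a candidate array and call DetectAndShoot, which moves candidates into the active target list by proximity, limited by NbTarget.
; A looping fire-rate timer line-traces to each active target.
; When a trace hits a BP_MoveChar, it spawns a following Bp_FireProjectil and applies damage immediately, without waiting for impact.
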(event `self.ReceiveBeginPlay`
  (`KismetArrayLibrary.Array_Clear` (`self.TargetsArray`)))

(event `Shoot`
  (bind _output (`|GetArrayItem` (`self.TargetLightning`) (`self.CurrentIndex`)))
  (if (not (`KismetSystemLibrary.K2_IsTimerActiveHandle` (`self.TimerShoot`)))
    (bind _returnvalue (`KismetSystemLibrary.K2_SetTimerDelegate` (delegate `Projectil`) (`self.FireRate_0`) true))
    (`/Engine/EditorBlueprintResources/StandardMacros.DoOnce` false
      (:`Completed`
        (set `self.TimerShoot` _returnvalue)
        (if (`self.HasTarget`) :!label _label
          (for (_array_element _array_index) (`self.TargetLightning`)
            (if (`KismetSystemLibrary.IsValid` _array_element)
              (set `self.CurrentIndex` _array_index)
              (bind _outhit (`KismetSystemLibrary.LineTraceSingle` :`Start` (`SceneComponent.K2_GetComponentLocation` (`self.Spawn`)) :`End` (`self.K2_GetActorLocation` _array_element) :`TraceChannel` "TraceTypeQuery1" :`DrawDebugType` "ForDuration"))
              (cast `/Game/Blueprints/BP_MoveChar` (`.HitActor` (`GameplayStatics.BreakHitResult` _outhit)))
              (bind _returnvalue_2 (`|SpawnActorFromClass` "/Game/Blueprints/Turrets/Projectiles/Bp_FireProjectil.Bp_FireProjectil_C" (`SceneComponent.K2_GetComponentToWorld` (`self.Spawn`)) "AdjustIfPossibleButAlwaysSpawn" "OverrideRootScale" null null))
              (`/Game/Blueprints/Turrets/Projectiles/Bp_FireProjectil.Follow` _returnvalue_2 _output)
              (`self.UpdateHealth` _output (`self.Damage`)))))))))

(event `Projectil`
  (goto _label))

(event `self.DetectionSphere.OnComponentBeginOverlap`
  (params (OverlappedComponent :type "PrimitiveComponent Object Reference") (OtherActor :type "Actor Object Reference") (OtherComp :type "PrimitiveComponent Object Reference") (OtherBodyIndex :type Integer) (bFromSweep :type Boolean) (SweepResult :type "HitResult Structure (by ref)"))
  (bind _targetsarray (`self.TargetsArray`))
  (bind _asbp_move_char (cast `/Game/Blueprints/BP_MoveChar` OtherActor))
  (bind _returnvalue (`KismetArrayLibrary.Array_Add` _targetsarray _asbp_move_char))
  (message `/Game/Blueprints/IaGestion.SetID` (`|GetArrayItem` _targetsarray _returnvalue) _returnvalue)
  (if (not (`self.HasTarget`))
    (`self.DetectAndShoot` :!label _label_2)
    (elif (and (`self.HasTarget`) (< (`KismetArrayLibrary.Array_Length` (`self.TargetLightning`)) (`self.NbTarget`)))
      (goto _label_2))))

(event `self.DetectionSphere.OnComponentEndOverlap`
  (params (OverlappedComponent :type "PrimitiveComponent Object Reference") (OtherActor :type "Actor Object Reference") (OtherComp :type "PrimitiveComponent Object Reference") (OtherBodyIndex :type Integer))
  (bind _asbp_move_char (cast `/Game/Blueprints/BP_MoveChar` OtherActor))
  (for (_array_element _array_index) (`self.TargetLightning`)
    (`/Engine/EditorBlueprintResources/StandardMacros.IsValid` _array_element
      (:`Is Valid`
        (if (== (`/Game/Blueprints/BP_MoveChar.Index` _array_element) (`/Game/Blueprints/BP_MoveChar.Index` _asbp_move_char))
          (`KismetArrayLibrary.Array_Remove` (`self.TargetLightning`) _array_index)))))
  (if (`KismetArrayLibrary.Array_IsNotEmpty` (`self.TargetsArray`))
    (`self.DetectAndShoot`)
    (else
      (set `self.HasTarget` false)
      (`KismetArrayLibrary.Array_Clear` (`self.TargetsArray`))
      (`KismetArrayLibrary.Array_Clear` (`self.TargetLightning`)))))

(fn `Detect Closer`
  (locals (TempDist :type "Float (double-precision)" :default 9999999.0) (ReturnIndex :type Integer))
  (bind _targetsarray (`self.TargetsArray`))
  (bind _targetlightning (`self.TargetLightning`))
  (for _array_element _targetlightning
    (`/Engine/EditorBlueprintResources/StandardMacros.IsValid` _array_element
      (:`Is Not Valid`
        (`KismetArrayLibrary.Array_RemoveItem` _targetlightning _array_element))))
  (if (> (`KismetArrayLibrary.Array_Length` (`self.TargetsArray`)) 1)
    (for _ (range (`self.NbTarget`))
      (set `local.TempDist` 99999.0 :!label _label)
      (if (> (`KismetArrayLibrary.Array_Length` _targetsarray) 0)
        (for (_array_element_2 _array_index) _targetsarray
          (`/Engine/EditorBlueprintResources/StandardMacros.IsValid` _array_element_2
            (:`Is Valid`
              (bind _returnvalue (`self.GetDistanceTo` _array_element_2 self))
              (if (< _returnvalue (`local.TempDist`))
                (set `local.TempDist` _returnvalue)
                (set `local.ReturnIndex` _array_index)))))
        (if (<= (`KismetArrayLibrary.Array_Length` (`self.TargetLightning`)) (`self.NbTarget`))
          (`KismetArrayLibrary.Array_Add` (`self.TargetLightning`) (`|GetArrayItem` (`self.TargetsArray`) (`local.ReturnIndex`)))
          (`KismetArrayLibrary.Array_Remove` (`self.TargetsArray`) (`self.CurrentIndex`))
          (return))
        (else
          (return))))
    (else
      (goto _label))))

(fn `DetectAndShoot`
  (`self.Detect Closer`)
  (`self.Shoot`)
  (set `self.HasTarget` true))

(fn `UserConstructionScript`
  (`SphereComponent.SetSphereRadius` (`self.DetectionSphere`) (`self.RadiusDetection_0`) true))