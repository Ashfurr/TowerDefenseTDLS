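; Mortar turret projectile actor that launches toward a given actor and destroys itself on impact.
; The Follow event clears its turret reference and sets the ProjectileMovement velocity once toward the target's current position, scaled by Speed, with no continuous homing here.
; Any Sphere hit destroys it; hitting a BP_MoveChar first adds a Niagara component to the projectile itself, immediately before destruction.
; The graph applies no damage.
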(event `Follow`
  (params (FollowActor :type "Actor Object Reference"))
  (set `self.WhichIsMyTurret` null)
  (set `MovementComponent.Velocity` (* (`KismetMathLibrary.GetDirectionUnitVector` (`self.K2_GetActorLocation`) (`self.K2_GetActorLocation` FollowActor)) (`self.Speed`)) (`self.ProjectileMovement`)))

(event `self.Sphere.OnComponentHit`
  (params (HitComponent :type "PrimitiveComponent Object Reference") (OtherActor :type "Actor Object Reference") (OtherComp :type "PrimitiveComponent Object Reference") (NormalImpulse :type "Vector Structure") (Hit :type "HitResult Structure (by ref)"))
  (cast `/Game/Blueprints/BP_MoveChar` OtherActor
    (:`then`
      (`AddComponent|NODE_AddNiagaraComponent-3`)
      (`self.K2_DestroyActor`))
    (:`CastFailed`
      (`self.K2_DestroyActor`))))

(fn `UserConstructionScript`)