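; Game mode for what appears to be a tower game, owning the player's life count and HUD.
; On BeginPlay it creates the WB_HUD widget, keeps a reference and adds it to the viewport.
; The UpdateHealthGM event decrements Life while it is above zero and pushes the value to the HUD's Health, printing a life-lost message, or prints a long-lasting defeat message once no lives remain.
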(event `self.ReceiveBeginPlay`
  (bind _returnvalue (`|CreateWidget` "/Game/UI/WB_HUD.WB_HUD_C"))
  (bind _output_get (set `self.HUDRef` _returnvalue))
  (`UserWidget.AddToViewport` _output_get 0))

(event `UpdateHealthGM`
  (bind _life (`self.Life`))
  (if (> _life 0)
    (bind _result (`/Engine/EditorBlueprintResources/StandardMacros.DecrementInt` _life)
      (:`  `
        (set `/Game/UI/WB_HUD.Health` (`KismetMathLibrary.Conv_IntToDouble` _result) (`self.HUDRef`))
        (`KismetSystemLibrary.PrintString` "vie perdu")))
    (else
      (`KismetSystemLibrary.PrintString` "ta perdue pd" true true (struct :`G` 0.66 :`B` 1.0 :`A` 1.0) 900.0))))

(fn `UserConstructionScript`)